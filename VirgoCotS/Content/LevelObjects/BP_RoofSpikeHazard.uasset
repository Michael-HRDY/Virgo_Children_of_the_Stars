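; Falling icicle hazard that drops once when a player-tagged actor enters its trigger box.
; BeginPlay places the icicle at StartHeight and takes the box's bottom as EndHeight.
; A timeline moves it between those heights via FInterpTo, with play rate inversely scaled by drop distance.
; Any overlap with the icicle destroys the actor, first applying damage and printing a message if a player is hit.
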(event `self.ReceiveBeginPlay`
  (bind _icicle (`self.Icicle`))
  (bind (_returnvalue_x _returnvalue_y) (`KismetMathLibrary.BreakVector` (`SceneComponent.K2_GetComponentLocation` _icicle)))
  (set `self.EndHeight` (- (.z (`SceneComponent.K2_GetComponentLocation` (`self.Box`))) (.z (`BoxComponent.GetScaledBoxExtent` (`self.Box`)))))
  (`SceneComponent.K2_SetWorldLocation` _icicle (`KismetMathLibrary.MakeVector` _returnvalue_x _returnvalue_y (`self.StartHeight`)) false false))

(event `self.Box.OnComponentBeginOverlap`
  (params (OverlappedComponent :type "PrimitiveComponent Object Reference") (OtherActor :type "Actor Object Reference") (OtherComp :type "PrimitiveComponent Object Reference") (OtherBodyIndex :type Integer) (bFromSweep :type Boolean) (SweepResult :type "HitResult Structure (by ref)"))
  (bind _icicle (`self.Icicle`))
  (bind (_returnvalue_x _returnvalue_y) (`KismetMathLibrary.BreakVector` (`SceneComponent.K2_GetComponentLocation` _icicle)))
  (if (`self.ActorHasTag` OtherActor "Player")
    (`/Engine/EditorBlueprintResources/StandardMacros.DoOnce` false
      (:`Completed`
        (`TimelineComponent.SetPlayRate` (`self.FallingIcicle`) (/ 1000.0 (* 1.75 (- (`self.StartHeight`) (`self.EndHeight`)))))
        (bind (_direction _timer) (`Timeline|FallingIcicle`)
          (:`Update`
            (`SceneComponent.K2_SetWorldLocation` _icicle (`KismetMathLibrary.MakeVector` _returnvalue_x _returnvalue_y (`KismetMathLibrary.FInterpTo` (`self.StartHeight`) (`self.EndHeight`) _timer 1.0)) false false)))))))

(event `self.Icicle.OnComponentBeginOverlap`
  (params (OverlappedComponent :type "PrimitiveComponent Object Reference") (OtherActor :type "Actor Object Reference") (OtherComp :type "PrimitiveComponent Object Reference") (OtherBodyIndex :type Integer) (bFromSweep :type Boolean) (SweepResult :type "HitResult Structure (by ref)"))
  (if (`self.ActorHasTag` OtherActor "Player")
    (`GameplayStatics.ApplyDamage` OtherActor 1.0)
    (`KismetSystemLibrary.PrintString` "Ouch"))
  (`self.K2_DestroyActor`))

(fn `UserConstructionScript`)